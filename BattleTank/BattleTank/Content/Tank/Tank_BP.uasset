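; Tank Blueprint over C++ logic that handles setup, camera orbit input and firing for a tank.
; BeginPlay passes the Barrel and Turret components to the SetBarrelReference and SetTurretReference functions, then assigns their static meshes.
; Aim axes rotate AzimuthGimbal in yaw and SpringArm in pitch separately, scaled by delta seconds for frame-rate independence.
; The Fire action calls Fire on press.
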(event `self.ReceiveBeginPlay`
  ;[1 1 1] Tank Set Mesh with C++ files
  (`self.SetBarrelReference` (`self.Barrel`))
  (`self.SetTurretReference` (`self.Turret`))
  (`StaticMeshComponent.SetStaticMesh` (`self.Turret`) "/Game/Tank/tank_fbx_Turret.tank_fbx_Turret")
  (`StaticMeshComponent.SetStaticMesh` (`self.Barrel`) "/Game/Tank/tank_fbx_Barrel.tank_fbx_Barrel"))

(event `InputAxis|AimAzimuth`
  (params (AxisValue :type "Float (single-precision)"))
  ;[1 1 1] Input Binding
  ;;[1 1 1] AimAzimuth Setup
  (`SceneComponent.K2_AddLocalRotation` (`self.Azimuth Gimbal`) (`KismetMathLibrary.MakeRotator` 0.0 0.0 (* AxisValue (`GameplayStatics.GetWorldDeltaSeconds`) 100.0)) false false))

(event `InputAxis|AimElevation`
  (params (AxisValue :type "Float (single-precision)"))
  ;[1 1 1] Input Binding
  ;;[1 1 1] AimElevation Setup
  (`SceneComponent.K2_AddLocalRotation` (`self.SpringArm`) (`KismetMathLibrary.MakeRotator` 0.0 (* AxisValue (`GameplayStatics.GetWorldDeltaSeconds`) 100.0)) false false))

(event `InputAction|Fire`
  (params (Key :type "Key Structure"))
  ;[1 1 1] Input Binding
  ;;[1 1 1] Fire Setup
  (:`Pressed`
    (`self.Fire`)))

(fn `UserConstructionScript`)